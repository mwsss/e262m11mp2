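; BP_CHpc04 is a player-controlled character that moves, shoots projectiles and toggles its mesh visibility.
; The MoveForward axis drives half-scale, reversed movement along the actor's right vector.
; V and left click pass through Sv then SvMc events, named like server-to-multicast relays, to flip StaticMesh visibility or spawn BP_PR_tama01 at the Arrow transform.
; Overlaps on StaticMesh call svHello, which prints a debug greeting.
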(event OnComponentBeginOverlap(StaticMesh)
  (params (OverlappedComponent :type Primitive%20Component%20Object%20Reference) (OtherActor :type Actor%20Object%20Reference) (OtherComp :type Primitive%20Component%20Object%20Reference) (OtherBodyIndex :type Integer) (bFromSweep :type Boolean) (SweepResult :type Hit%20Result%20Structure%20%28by%20ref%29))
  (CallFunction|SvHello))

(event Custom|svTama
  (params (acTrnsf :type Transform))
  (CallFunction|SvMcTama acTrnsf))

(event Custom|svMcTama
  (params (acTmsf :type Transform))
  (Game|SpawnActorfromClass "/Game/BP/GIMIC/BP_PR_tama01.BP_PR_tama01_C" acTmsf "Undefined" 0 0))

(event Custom|svHello
  (Development|PrintString "Hello"))

(event Custom|svSetvis
  (CallFunction|SvMcSetv))

(event Custom|svMcSetv
  (bind _isa (Utilities|FlowControl|FlipFlop)
    (:A
      _)
    (:B
      _))
  (Rendering|SetVisibility (Variables|Default|GetStaticMesh) _isa false))

(event EventBeginPlay)

(event Collision|EventActorBeginOverlap
  (params (OtherActor :type Actor%20Object%20Reference)))

(event EventTick
  (params (DeltaSeconds :type Float%20%28single-precision%29)))

(event Input|AxisEvents|InputAxisMoveForward
  (params (AxisValue :type Float%20%28single-precision%29))
  (Pawn|Input|AddMovementInput (Transformation|GetActorRightVector) (* AxisValue -0.5) false))

(event Input|MouseEvents|LeftMouseButton
  (params (Key :type Key%20Structure :default "None"))
  (:Pressed
    (CallFunction|SvTama (Transformation|GetWorldTransform (Variables|Default|GetArrow)))))

(event Input|KeyboardEvents|V
  (params (Key :type Key%20Structure :default "None"))
  (:Pressed
    (CallFunction|SvSetvis)))

(fn ConstructionScript)