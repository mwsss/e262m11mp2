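; BP_spu02 is a moving-floor gimmick that carries a static mesh along a spline after its trigger box is overlapped.
; Any overlap on the box sets a three-second timer that fires the IdouYuka event.
; IdouYuka re-calls itself after short delays, stepping SpNow and placing the mesh at that spline time without sweep.
; The actor destroys itself once SpNow reaches the spline's duration.
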(event OnComponentBeginOverlap(Box)
  (params (OverlappedComponent :type Primitive%20Component%20Object%20Reference) (OtherActor :type Actor%20Object%20Reference) (OtherComp :type Primitive%20Component%20Object%20Reference) (OtherBodyIndex :type Integer) (bFromSweep :type Boolean) (SweepResult :type Hit%20Result%20Structure%20%28by%20ref%29))
  (Utilities|Time|SetTimerbyEvent (delegate Custom|idouYuka) 3.0))

(event Custom|idouYuka
  (bind _spline (Variables|Default|GetSpline))
  (if (< (Variables|Default|GetspNow) (Variables|/Script/Engine.SplineComponent|GetDuration _spline))
    (Utilities|FlowControl|Delay 0.01)
    (bind _output_get (Variables|Default|SetspNow (+ (Variables|Default|GetspNow) 0.01)))
    (Transformation|SetWorldLocation (Variables|Default|GetStaticMesh) (Spline|GetLocationatTime _spline _output_get "World" false) false false)
    (CallFunction|IdouYuka)
    (else
      (Actor|DestroyActor))))

(fn ConstructionScript)